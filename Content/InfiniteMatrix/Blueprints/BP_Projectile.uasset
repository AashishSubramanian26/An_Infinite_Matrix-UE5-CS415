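; BP_Projectile is a projectile actor that destroys enemies and awards the player score.
; It caches the player pawn at BeginPlay and moves with a ProjectileMovement component.
; When its sphere hits anything but the player, it destroys itself, and a hit BP_Enemy is also destroyed and adds a point.
; Every fifth point raises the player's forward speed; the logic assigning ProjectileSpeed to the movement component is disconnected.
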(event OnComponentHit(Sphere)
  (params (HitComponent :type Primitive%20Component%20Object%20Reference) (OtherActor :type Actor%20Object%20Reference) (OtherComp :type Primitive%20Component%20Object%20Reference) (NormalImpulse :type Vector :default "0, 0, 0") (Hit :type Hit%20Result%20Structure%20%28by%20ref%29))
  (bind _player_reference (Variables|Default|GetPlayer%20Reference))
  (Utilities|Casting|CastToBP_Player OtherActor
    (:CastFailed
      (Actor|DestroyActor)
      (bind _asbp_enemy (Utilities|Casting|CastToBP_Enemy OtherActor))
      (Actor|DestroyActor _asbp_enemy)
      (Utilities|IsValid (Variables|Default|GetPlayer%20Reference)
        (:Is%20Valid
          (Variables|/Game/InfiniteMatrix/Blueprints/BP_Player.BP_Player_C|SetScore _player_reference (+ (Variables|/Game/InfiniteMatrix/Blueprints/BP_Player.BP_Player_C|GetScore _player_reference) 1))
          (if (== (Math|Integer|%(Integer) (Variables|/Game/InfiniteMatrix/Blueprints/BP_Player.BP_Player_C|GetScore _player_reference) 5) 0)
            (Variables|/Game/InfiniteMatrix/Blueprints/BP_Player.BP_Player_C|SetForwardSpeed _player_reference (+ (Variables|/Game/InfiniteMatrix/Blueprints/BP_Player.BP_Player_C|GetForwardSpeed _player_reference) 1.5e+02))))))))

(event OnComponentActivated(ProjectileMovement)
  (params (Component :type Actor%20Component%20Object%20Reference) (bReset :type Boolean)))

(event EventBeginPlay
  (bind _asbp_player (Utilities|Casting|CastToBP_Player (Game|Player|GetPlayerPawn 0)))
  (Variables|Default|SetPlayer%20Reference _asbp_player))

(event Collision|EventActorBeginOverlap
  (params (OtherActor :type Actor%20Object%20Reference)))

(event EventTick
  (params (DeltaSeconds :type Float%20%28single-precision%29)))

(fn ConstructionScript)