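; BP_HealthPack is a pickup that restores one point of health when the player overlaps its Cube component.
; On overlap it raises BP_Player's CurrentHealth by one and plays a sound, unless health is already at the cap, and destroys itself either way.
; Tick compares the cached player's X position with its own and destroys the pack once the player has moved past it.
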(event OnComponentBeginOverlap(Cube)
  (params (OverlappedComponent :type Primitive%20Component%20Object%20Reference) (OtherActor :type Actor%20Object%20Reference) (OtherComp :type Primitive%20Component%20Object%20Reference) (OtherBodyIndex :type Integer) (bFromSweep :type Boolean) (SweepResult :type Hit%20Result%20Structure%20%28by%20ref%29))
  ;[1 1 1] When the player collides with this, we are going to increase the players health by 1
  (bind _asbp_player (Utilities|Casting|CastToBP_Player OtherActor))
  ;[1 1 1] Checking that we can't make our health more thats allowed
  (if (>= (Variables|/Game/InfiniteMatrix/Blueprints/BP_Player.BP_Player_C|GetCurrentHealth _asbp_player) 3.0)
    (Variables|/Game/InfiniteMatrix/Blueprints/BP_Player.BP_Player_C|SetCurrentHealth _asbp_player (Variables|/Game/InfiniteMatrix/Blueprints/BP_Player.BP_Player_C|GetCurrentHealth _asbp_player))
    (else
      (Variables|/Game/InfiniteMatrix/Blueprints/BP_Player.BP_Player_C|SetCurrentHealth _asbp_player (+ (Variables|/Game/InfiniteMatrix/Blueprints/BP_Player.BP_Player_C|GetCurrentHealth _asbp_player) 1.0))
      (Audio|PlaySound2D "/Game/InfiniteMatrix/Audio/AUD_HealthUp.AUD_HealthUp" 1.0 1.0 0.0 0 0)))
  (Actor|DestroyActor))

(event EventBeginPlay
  (bind _asbp_player (Utilities|Casting|CastToBP_Player (Game|Player|GetPlayerPawn 0)))
  (Variables|Default|SetPlay%20Ref _asbp_player))

(event EventTick
  (params (DeltaSeconds :type Float%20%28single-precision%29))
  (if (> (.x (Transformation|GetWorldLocation (Variables|/Script/Engine.Actor|GetRootComponent (Variables|Default|GetPlay%20Ref)))) (.x (Transformation|GetActorLocation)))
    (Actor|DestroyActor)))

(fn ConstructionScript)