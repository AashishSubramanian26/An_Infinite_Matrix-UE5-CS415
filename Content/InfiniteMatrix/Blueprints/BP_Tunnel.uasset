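; Endless tunnel segment with a spinning, holed wall the player must fly through.
; Passing its trigger adds score unless the wall was hit, requests the next segment, destroys this one and boosts speed at multiples of five.
; Wall hits cost health, then either recolor the tunnel and disable wall collision, or kill the player, clearing pickups and enemies.
; Helper functions randomize the wall and spawn health packs and enemies.
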(event OnComponentBeginOverlap(TriggerZone)
  (params (OverlappedComponent :type Primitive%20Component%20Object%20Reference) (OtherActor :type Actor%20Object%20Reference) (OtherComp :type Primitive%20Component%20Object%20Reference) (OtherBodyIndex :type Integer) (bFromSweep :type Boolean) (SweepResult :type Hit%20Result%20Structure%20%28by%20ref%29))
  ;[1 1 1] Section where we increase our score and speed when needed
  (bind _asbp_player (Utilities|Casting|CastToBP_Player OtherActor))
  (if (Variables|Default|GetIsHit)
    ;;[1 1 1] If you hit something, tthe score will not increase, but if you didn't, score will increase
    (Variables|/Game/InfiniteMatrix/Blueprints/BP_Player.BP_Player_C|SetScore _asbp_player (Variables|/Game/InfiniteMatrix/Blueprints/BP_Player.BP_Player_C|GetScore _asbp_player))
    (else
      (Variables|/Game/InfiniteMatrix/Blueprints/BP_Player.BP_Player_C|SetScore _asbp_player (+ (Variables|/Game/InfiniteMatrix/Blueprints/BP_Player.BP_Player_C|GetScore _asbp_player) 1))))
  (Default|SpawnTunnelatSpawnPoint (Variables|Default|GetTunnelSpawner))
  (Actor|DestroyActor)
  (if (== (Math|Integer|%(Integer) (Variables|/Game/InfiniteMatrix/Blueprints/BP_Player.BP_Player_C|GetScore _asbp_player) 5) 0)
    (Variables|/Game/InfiniteMatrix/Blueprints/BP_Player.BP_Player_C|SetForwardSpeed _asbp_player (+ (Variables|/Game/InfiniteMatrix/Blueprints/BP_Player.BP_Player_C|GetForwardSpeed _asbp_player) 1.5e+02))))

(event OnComponentHit(WallMesh)
  (params (HitComponent :type Primitive%20Component%20Object%20Reference) (OtherActor :type Actor%20Object%20Reference) (OtherComp :type Primitive%20Component%20Object%20Reference) (NormalImpulse :type Vector :default "0, 0, 0") (Hit :type Hit%20Result%20Structure%20%28by%20ref%29))
  ;[1 1 1] Section for when we hit the wall
  (bind _asbp_player (Utilities|Casting|CastToBP_Player OtherActor))
  (Variables|Default|SetIsHit true)
  ;;[1 1 1] Get the current health and check if it <= 0, if true, then player needs to die
  (bind _output_get (Variables|/Game/InfiniteMatrix/Blueprints/BP_Player.BP_Player_C|SetCurrentHealth _asbp_player (- (Variables|/Game/InfiniteMatrix/Blueprints/BP_Player.BP_Player_C|GetCurrentHealth _asbp_player) 1.0)))
  (if (<= _output_get 0.0)
    (Variables|/Game/InfiniteMatrix/Blueprints/BP_Player.BP_Player_C|SetIsDead _asbp_player true)
    (Collision|SetCollisionProfileName (Variables|Default|GetWallMesh) "BlockAllDynamic" true :!class /Script/Engine.PrimitiveComponent)
    (Camera|PlayWorldCameraShake "/Game/InfiniteMatrix/Blueprints/BP_CameraShake.BP_CameraShake_C" (Transformation|GetActorLocation _asbp_player) 0.0 5e+02)
    (Audio|PlaySound2D "/Game/InfiniteMatrix/Audio/AUD_Damage.AUD_Damage" 1.0 1.0 0.0 0 0)
    (bind _outactors (Actor|GetAllActorsOfClass "/Game/InfiniteMatrix/Blueprints/BP_HealthPack.BP_HealthPack_C"))
    (for _array_element _outactors
      (Actor|DestroyActor _array_element))
    (bind _outactors_2 (Actor|GetAllActorsOfClass "/Game/InfiniteMatrix/Blueprints/BP_Enemy.BP_Enemy_C"))
    (for _array_element_2 _outactors_2
      (Actor|DestroyActor _array_element_2))
    (Default|DisplayRestart _asbp_player)
    (else
      (Collision|SetCollisionProfileName (Variables|Default|GetWallMesh) "NoCollision" true :!class /Script/Engine.PrimitiveComponent)
      (Rendering|Material|SetMaterial (Variables|Debug|GetStaticMeshComponent) 0 (Utilities|Select :Index (Math|Integer|%(Integer) (Math|Float|Truncate (Variables|/Game/InfiniteMatrix/Blueprints/BP_Player.BP_Player_C|GetCurrentHealth _asbp_player)) 3) :Option%200 "/Game/InfiniteMatrix/Materials/MI_TunnelHealth3.MI_TunnelHealth3" :Option%201 "/Game/InfiniteMatrix/Materials/MI_TunnelHealth1.MI_TunnelHealth1" :Option%202 "/Game/InfiniteMatrix/Materials/MI_TunnelHealth2.MI_TunnelHealth2"))
      (Camera|PlayWorldCameraShake "/Game/InfiniteMatrix/Blueprints/BP_CameraShake.BP_CameraShake_C" (Transformation|GetActorLocation _asbp_player) 0.0 5e+02)
      (Audio|PlaySound2D "/Game/InfiniteMatrix/Audio/AUD_Damage.AUD_Damage" 1.0 1.0 0.0 0 0))))

(event EventBeginPlay
  (bind _returnvalue (Actor|GetActorOfClass "/Game/InfiniteMatrix/Blueprints/BP_Projectile.BP_Projectile_C"))
  (bind _asbp_projectile (Utilities|Casting|CastToBP_Projectile _returnvalue))
  (Variables|Default|SetProjectile%20Reference _asbp_projectile))

(event EventTick
  (params (DeltaSeconds :type Float%20%28single-precision%29))
  (Transformation|AddLocalRotation (Variables|Default|GetWallMesh) (Math|Rotator|MakeRotator (* DeltaSeconds (Variables|Default|GetRotate%20Speed)) 0.0 0.0) false false))

(fn ConstructionScript)

(fn RandomizeWall
  (Components|StaticMesh|SetStaticMesh (Variables|Default|GetWallMesh) (Utilities|Select :Index (Math|Random|RandomIntegerinRange 0 3) :Option%200 "/Game/InfiniteMatrix/Meshes/SM_Hole_01.SM_Hole_01" :Option%201 "/Game/InfiniteMatrix/Meshes/SM_Hole_02.SM_Hole_02" :Option%202 "/Game/InfiniteMatrix/Meshes/SM_Hole_03.SM_Hole_03" :Option%203 "/Game/InfiniteMatrix/Meshes/SM_Hole_04.SM_Hole_04"))
  (Transformation|AddLocalRotation (Variables|Default|GetWallMesh) (Math|Rotator|MakeRotator (Math|Random|RandomFloatinRange 0.0 3.6e+02) 0.0 0.0) false false))

(fn RandomizeHealthPack
  (params (Spawn%20Location :type Vector))
  (if (== (Math|Random|RandomIntegerinRange 0 3) 0)
    (Game|SpawnActorfromClass "/Game/InfiniteMatrix/Blueprints/BP_HealthPack.BP_HealthPack_C" (Math|Transform|MakeTransform (Math|Vector|MakeVector (- (.x Spawn%20Location) (Math|Random|RandomIntegerinRange 750 1900)) (- (.y Spawn%20Location) (Math|Random|RandomIntegerinRange -200 200)) (- (.z Spawn%20Location) (Math|Random|RandomIntegerinRange -200 200))) "0, 0, 0" "1.000000,1.000000,1.000000") "Undefined" "MultiplyWithRoot" 0 0)))

(fn ChangeTunnelColor
  (Rendering|Material|SetMaterial (Variables|Debug|GetStaticMeshComponent) 0 (Utilities|Select :Index 0 :Option%200 "/Game/InfiniteMatrix/Materials/MI_TunnelHealth3.MI_TunnelHealth3" :Option%201 "/Game/InfiniteMatrix/Materials/MI_TunnelHealth2.MI_TunnelHealth2" :Option%202 "/Game/InfiniteMatrix/Materials/MI_TunnelHealth1.MI_TunnelHealth1")))

(fn RandomizeEnemy
  (params (Location :type Vector))
  (if (== (Math|Random|RandomIntegerinRange 0 0) 0)
    (Game|SpawnActorfromClass "/Game/InfiniteMatrix/Blueprints/BP_Enemy.BP_Enemy_C" (Math|Transform|MakeTransform (Math|Vector|MakeVector (- (.x Location) (Math|Random|RandomIntegerinRange 900 1900)) (- (.y Location) (Math|Random|RandomIntegerinRange -200 200)) (- (.z Location) (Math|Random|RandomIntegerinRange -200 200))) "0, 0, 0" "1.000000,1.000000,1.000000") "Undefined" "MultiplyWithRoot" 0 0)))