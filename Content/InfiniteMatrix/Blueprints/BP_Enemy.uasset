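; BP_Enemy is a hazard actor that damages BP_Player when its Cone component is overlapped.
; It caches the player on BeginPlay and destroys itself on Tick once the player's X position exceeds its own.
; On a hit it destroys itself, removes one health point and plays a camera shake and damage sound.
; At zero health it also flags the player dead, clears all health packs and enemies, and calls the player's DisplayRestart.
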(event OnComponentBeginOverlap(Cone)
  (params (OverlappedComponent :type Primitive%20Component%20Object%20Reference) (OtherActor :type Actor%20Object%20Reference) (OtherComp :type Primitive%20Component%20Object%20Reference) (OtherBodyIndex :type Integer) (bFromSweep :type Boolean) (SweepResult :type Hit%20Result%20Structure%20%28by%20ref%29))
  (bind _asbp_player (Utilities|Casting|CastToBP_Player OtherActor))
  (Actor|DestroyActor)
  ;[1 1 1] Get the current health and check if it <= 0, if true, then player needs to die
  (bind _output_get (Variables|/Game/InfiniteMatrix/Blueprints/BP_Player.BP_Player_C|SetCurrentHealth _asbp_player (- (Variables|/Game/InfiniteMatrix/Blueprints/BP_Player.BP_Player_C|GetCurrentHealth _asbp_player) 1.0)))
  (if (<= _output_get 0.0)
    (Variables|/Game/InfiniteMatrix/Blueprints/BP_Player.BP_Player_C|SetIsDead _asbp_player true)
    (Camera|PlayWorldCameraShake "/Game/InfiniteMatrix/Blueprints/BP_CameraShake.BP_CameraShake_C" (Transformation|GetActorLocation _asbp_player) 0.0 5e+02)
    (Audio|PlaySound2D "/Game/InfiniteMatrix/Audio/AUD_Damage.AUD_Damage" 1.0 1.0 0.0 0 0)
    (bind _outactors (Actor|GetAllActorsOfClass "/Game/InfiniteMatrix/Blueprints/BP_HealthPack.BP_HealthPack_C"))
    (for _array_element _outactors
      (Actor|DestroyActor _array_element))
    (bind _outactors_2 (Actor|GetAllActorsOfClass "BP_Enemy_C"))
    (for _array_element_2 _outactors_2
      (Actor|DestroyActor _array_element_2))
    (Default|DisplayRestart _asbp_player)
    (else
      (Camera|PlayWorldCameraShake "/Game/InfiniteMatrix/Blueprints/BP_CameraShake.BP_CameraShake_C" (Transformation|GetActorLocation _asbp_player) 0.0 5e+02)
      (Audio|PlaySound2D "/Game/InfiniteMatrix/Audio/AUD_Damage.AUD_Damage" 1.0 1.0 0.0 0 0))))

(event EventBeginPlay
  (bind _asbp_player (Utilities|Casting|CastToBP_Player (Game|Player|GetPlayerPawn 0)))
  (Variables|Default|SetPlay%20Ref _asbp_player))

(event Collision|EventActorBeginOverlap
  (params (OtherActor :type Actor%20Object%20Reference)))

(event EventTick
  (params (DeltaSeconds :type Float%20%28single-precision%29))
  (if (> (.x (Transformation|GetWorldLocation (Variables|/Script/Engine.Actor|GetRootComponent (Variables|Default|GetPlay%20Ref)))) (.x (Transformation|GetActorLocation)))
    (Actor|DestroyActor)))

(fn ConstructionScript)